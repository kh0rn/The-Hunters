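; Biter enemy actor that runs a struggle quick-time event when the player enters its BiteVolume.
; The overlap freezes player movement, registers itself on the character, blends to its camera and shows a press widget.
; Tick raises Power, driving camera shake, red tint and vignette, while Push lowers it until either limit stops the bite.
; Externally triggered DeadBody and Escape events remove the widget and return the view, killing or releasing the player.
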(event `DeadBody`
  (bind _returnvalue (`GameplayStatics.GetPlayerCharacter` 0))
  (`Widget.RemoveFromParent` (`self.Widget`))
  (bind _asfirst_person_character (cast `/Game/FirstPersonCPP/Blueprints/FirstPersonCharacter` _returnvalue))
  (`/Game/FirstPersonCPP/Blueprints/FirstPersonCharacter.Dead` _asfirst_person_character)
  (`GameplayStatics.PlayWorldCameraShake` "/Game/QT/Dead_CS.Dead_CS_C" (`SceneComponent.K2_GetComponentLocation` (`/Game/FirstPersonCPP/Blueprints/FirstPersonCharacter.CameraDead` _asfirst_person_character)) 1.0 1.0)
  (`PlayerController.SetViewTargetWithBlend` (`GameplayStatics.GetPlayerController` 0) _returnvalue 1.0 "VTBlend_Linear" 0.0 false))

(event `Escape`
  (bind _returnvalue (`GameplayStatics.GetPlayerController` 0))
  (bind _returnvalue_2 (`GameplayStatics.GetPlayerCharacter` 0))
  (`Widget.RemoveFromParent` (`self.Widget`))
  (`PlayerController.SetViewTargetWithBlend` _returnvalue _returnvalue_2 0.5 "VTBlend_Linear" 0.0 false)
  (`self.EnableInput` _returnvalue_2 _returnvalue)
  (set `CharacterMovementComponent.MaxWalkSpeed` 600.0 (`Character.CharacterMovement` _returnvalue_2)))

(event `self.ReceiveTick`
  (params (DeltaSeconds :type "Float (single-precision)"))
  (bind _returnvalue (/ (`self.Power`) 100.0))
  (bind _returnvalue_2 (+ (`self.Power`) (* DeltaSeconds (`self.BiteRate`))))
  (if (`self.bBite`)
    (set `self.Power` _returnvalue_2)
    (`GameplayStatics.PlayWorldCameraShake` "/Game/QT/Bite_CS.Bite_CS_C" (`SceneComponent.K2_GetComponentLocation` (`self.CameraBite`)) 0.5 0.5)
    (bind _structout (setmembers `PostProcessSettings` :`StructRef` (make `PostProcessSettings` :`SceneColorTint` (`KismetMathLibrary.LinearColorLerp` (struct :`R` 1.0 :`G` 1.0 :`B` 1.0) (struct :`R` 1.0 :`A` 0.5) _returnvalue) :`VignetteIntensity` _returnvalue)))
    (set `CameraComponent.PostProcessSettings` _structout (`self.CameraBite`))
    (if (>= _returnvalue_2 100.0)
      (set `self.Power` 100.0)
      (set `self.bBite` false)
      (elif (<= _returnvalue_2 0.0)
        (set `self.Power` 0.0)
        (set `self.bBite` false)))))

(event `self.BiteVolume.OnComponentBeginOverlap`
  (params (OverlappedComponent :type "PrimitiveComponent Object Reference") (OtherActor :type "Actor Object Reference") (OtherComp :type "PrimitiveComponent Object Reference") (OtherBodyIndex :type Integer) (bFromSweep :type Boolean) (SweepResult :type "HitResult Structure (by ref)"))
  (bind _returnvalue (`GameplayStatics.GetPlayerController` 0))
  (bind _asfirst_person_character (cast `/Game/FirstPersonCPP/Blueprints/FirstPersonCharacter` OtherActor))
  (set `self.bBite` true)
  (`PlayerController.SetViewTargetWithBlend` _returnvalue self 0.5 "VTBlend_Linear" 0.0 false)
  (set `/Game/FirstPersonCPP/Blueprints/FirstPersonCharacter.Biter` self _asfirst_person_character)
  (set `CharacterMovementComponent.MaxWalkSpeed` 0.0 (`Character.CharacterMovement` _asfirst_person_character))
  (bind _returnvalue_2 (`|CreateWidget` "/Game/QT/Widget/Press_BP.Press_BP_C" _returnvalue))
  (`UserWidget.AddToViewport` _returnvalue_2 0)
  (set `self.Widget` _returnvalue_2))

(fn `Push`
  (params (PushPower :type "Float (double-precision)"))
  (if (< (`self.Power`) 100.0)
    (set `self.Power` (- (`self.Power`) PushPower))))

(fn `UserConstructionScript`)