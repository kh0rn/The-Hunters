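; Master weapon Blueprint that signals when a Hunter character is in range of the weapon.
; Overlap events on its Sphere component show a Widget and turn on the StaticMesh's custom depth when a Hunter enters, then reverse both on exit.
; The Player reference is cleared on entry and set to the Hunter on exit, the inverse of a usual in-range reference.
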(event `self.Sphere.OnComponentBeginOverlap`
  (params (OverlappedComponent :type "PrimitiveComponent Object Reference") (OtherActor :type "Actor Object Reference") (OtherComp :type "PrimitiveComponent Object Reference") (OtherBodyIndex :type Integer) (bFromSweep :type Boolean) (SweepResult :type "HitResult Structure (by ref)"))
  (cast `/Game/BP/Character/Hunter` OtherActor)
  (set `self.Player` null)
  (`SceneComponent.SetVisibility` (`self.Widget`) true false)
  (`PrimitiveComponent.SetRenderCustomDepth` (`self.StaticMesh`) true))

(event `self.Sphere.OnComponentEndOverlap`
  (params (OverlappedComponent :type "PrimitiveComponent Object Reference") (OtherActor :type "Actor Object Reference") (OtherComp :type "PrimitiveComponent Object Reference") (OtherBodyIndex :type Integer))
  (bind _ashunter (cast `/Game/BP/Character/Hunter` OtherActor))
  (set `self.Player` _ashunter)
  (`SceneComponent.SetVisibility` (`self.Widget`) false false)
  (`PrimitiveComponent.SetRenderCustomDepth` (`self.StaticMesh`) false))

(fn `UserConstructionScript`)