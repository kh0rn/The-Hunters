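; Eye actor Blueprint whose Eye component tracks the player's follow camera, so the eye appears to watch the player.
; BeginPlay casts player character 0 to Hunter, caching it along with the eye's starting rotation, which is not used afterward.
; Each Tick, MenagmentCamera computes the look-at rotation from camera to eye and applies it in world space with pitch offset by 180 degrees.
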(event `MenagmentCamera`
  (bind _hunter (`self.Hunter`))
  ;[1 1 1] Глаз следит за игроком
  (`/Engine/EditorBlueprintResources/StandardMacros.IsValid` _hunter
    (:`Is Valid`
      (`SceneComponent.K2_SetWorldRotation` (`self.Eye`) (`KismetMathLibrary.MakeRotator` (.roll (`KismetMathLibrary.FindLookAtRotation` (`SceneComponent.K2_GetComponentLocation` (`/Game/BP/Character/Hunter.FollowCamera` _hunter)) (`SceneComponent.K2_GetComponentLocation` (`self.Eye`)))) (- (.pitch (`KismetMathLibrary.FindLookAtRotation` (`SceneComponent.K2_GetComponentLocation` (`/Game/BP/Character/Hunter.FollowCamera` _hunter)) (`SceneComponent.K2_GetComponentLocation` (`self.Eye`)))) 180.0) (.yaw (`KismetMathLibrary.FindLookAtRotation` (`SceneComponent.K2_GetComponentLocation` (`/Game/BP/Character/Hunter.FollowCamera` _hunter)) (`SceneComponent.K2_GetComponentLocation` (`self.Eye`))))) false false))))

(event `self.ReceiveBeginPlay`
  ;[1 1 1] Настройка переменных
  (bind _ashunter (cast `/Game/BP/Character/Hunter` (`GameplayStatics.GetPlayerCharacter` 0)))
  (set `self.Hunter` _ashunter)
  (set `self.StartRotation` (`SceneComponent.K2_GetComponentRotation` (`self.Eye`))))

(event `self.ReceiveTick`
  (params (DeltaSeconds :type "Float (single-precision)"))
  (`self.MenagmentCamera`))

(fn `UserConstructionScript`)