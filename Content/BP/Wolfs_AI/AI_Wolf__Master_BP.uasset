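; Master wolf AI character that takes damage from the player, shows a health bar and dies into a ragdoll.
; BeginPlay fills health, binds the hidden Wolf_UI widget and attaches glowing eye emitters, while construction applies the configurable mesh.
; ITakeDamage reveals the bar and either kills instantly on a "Brust" bone hit or subtracts health and sets EnemyFound.
; EnableCombat plays the AI_seat montage in reverse as the attack.
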(event `self.ReceiveBeginPlay`
  (bind _mesh (`self.Mesh`))
  (bind _mesh_2 (`self.Mesh`))
  ;[1 1 1] Инициализация переменных, отображение полоски хелсбара
  (set `self.CurrentHealth` (`self.MaxHealth`))
  (bind _aswolf_ui (cast `/Game/UI/User/Wolf_UI` (`WidgetComponent.GetUserWidgetObject` (`self.Widget`))))
  (set `/Game/UI/User/Wolf_UI.Owner` self _aswolf_ui)
  (`SceneComponent.SetVisibility` (`self.Widget`) false false)
  ;[1 1 1] Установка эффекта для левого глаза
  (bind _returnvalue (`GameplayStatics.SpawnEmitterAttached` "/Game/fx/P_RedWolf.P_RedWolf" (`self.Mesh`) "EyeLeft" (`SceneComponent.GetSocketLocation` _mesh_2 "EyeLeft") (`SceneComponent.GetSocketRotation` _mesh_2 "EyeLeft") (0.06 0.06 0.06) "KeepWorldPosition" false))
  (set `self.EffectLeftEye` _returnvalue)
  ;[1 1 1] Установка эффекта для правого глаза
  (bind _returnvalue_2 (`GameplayStatics.SpawnEmitterAttached` "/Game/fx/P_RedWolf.P_RedWolf" (`self.Mesh`) "EyeRigth" (`SceneComponent.GetSocketLocation` _mesh "EyeRigth") (`SceneComponent.GetSocketRotation` _mesh "EyeRigth") (0.06 0.06 0.06) "KeepWorldPosition" false))
  (set `self.EffecRigthEye` _returnvalue_2))

(event `/Game/BP/Interfaces/TakeDamage.iTakeDamage`
  (params (BoneName :type Name) (Damage :type "Float (single-precision)"))
  ;[1 1 1] Получение урона от игрока
  ;;[1 1 1] Включить полоску ХП
  (`SceneComponent.SetVisibility` (`self.Widget`) true false)
  (if (== BoneName "Brust")
    (`KismetSystemLibrary.PrintString` "Head shot")
    (set `self.CurrentHealth` 0.0)
    (else
      (set `self.EnemyFound` true)
      (set `self.CurrentHealth` (- (`self.CurrentHealth`) Damage))))
  (if (<= (`self.CurrentHealth`) 0.0)
    ;;[1 1 1] Смерть AI
    (set `self.IsDeath` true)
    (`SkeletalMeshComponent.SetAllBodiesSimulatePhysics` (`self.Mesh`) true)
    (`PrimitiveComponent.SetCollisionEnabled` (`self.CapsuleComponent`) "NoCollision")
    (`SceneComponent.SetVisibility` (`self.Widget`) false false)
    (`SceneComponent.SetVisibility` (`self.EffecRigthEye`) false false)
    (`SceneComponent.SetVisibility` (`self.EffectLeftEye`) false false)))

(event `EnableCombat`
  ;[1 1 1] Анимация атаки
  (`self.PlayAnimMontage` "/Game/BP/Wolfs_AI/AnimationSmallWolf/AI_seat.AI_seat" -1.0))

(fn `UserConstructionScript`
  (`SkinnedMeshComponent.SetSkinnedAssetAndUpdate` (`self.Mesh`) (`self.MeshWolf`) true))