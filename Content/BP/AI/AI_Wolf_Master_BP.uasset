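; Master wolf AI character with health, a health bar widget, damage handling and ragdoll death.
; BeginPlay links the widget, caches the weather manager and attaches red particle effects to both eye sockets.
; Hits on the "Brust" bone kill instantly; others subtract health and flag the enemy as found.
; EnableCombat plays a montage in reverse; the sunset-based eye toggle is disconnected from Tick, so never runs.
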(event `self.ReceiveBeginPlay`
  (bind _mesh (`self.Mesh`))
  (bind _mesh_2 (`self.Mesh`))
  ;[1 1 1] Инициализация переменных, отображение полоски хелсбара
  (set `self.CurrentHealth` (`self.MaxHealth`))
  (bind _aswolf_ui (cast `/Game/UI/User/Wolf_UI` (`WidgetComponent.GetUserWidgetObject` (`self.Widget`))))
  (set `/Game/UI/User/Wolf_UI.Owner` self _aswolf_ui)
  (`SceneComponent.SetVisibility` (`self.Widget`) (`self.SeeHealth`) false)
  (bind _outactors (`GameplayStatics.GetAllActorsOfClass` "/Game/BP/Weather/WeatherManager_BP.WeatherManager_BP_C"))
  (bind _output (`|GetArrayItem` _outactors))
  (cast `/Game/BP/Weather/WeatherManager_BP` _output)
  ;[1 1 1] Установка эффекта для левого глаза
  (set `self.WeatherManager` _output)
  (bind _returnvalue (`GameplayStatics.SpawnEmitterAttached` "/Game/fx/P_RedWolf.P_RedWolf" (`self.Mesh`) "EyeLeft" (`SceneComponent.GetSocketLocation` _mesh_2 "EyeLeft") (`SceneComponent.GetSocketRotation` _mesh_2 "EyeLeft") (0.0006 0.0006 0.0006) "KeepWorldPosition" false))
  (bind _output_get (set `self.EffectLeftEye` _returnvalue))
  (`SceneComponent.SetVisibility` _output_get true false)
  ;[1 1 1] Установка эффекта для правого глаза
  (bind _returnvalue_2 (`GameplayStatics.SpawnEmitterAttached` "/Game/fx/P_RedWolf.P_RedWolf" (`self.Mesh`) "EyeRigth" (`SceneComponent.GetSocketLocation` _mesh "EyeLeft") (`SceneComponent.GetSocketRotation` _mesh "EyeLeft") (1.0 1.0 1.0) "KeepWorldPosition" false))
  (bind _output_get_2 (set `self.EffecRigthEye` _returnvalue_2))
  (`SceneComponent.SetVisibility` _output_get_2 true false))

(event `/Game/BP/AI/TakeDamage.iTakeDamage`
  (params (BoneName :type Name) (Damage :type "Float (single-precision)"))
  ;[1 1 1] Получение урона от игрока
  (if (== BoneName "Brust")
    (`KismetSystemLibrary.PrintString` "Head shot")
    (set `self.CurrentHealth` 0.0)
    (else
      (set `self.EnemyFound` true)
      (set `self.CurrentHealth` (- (`self.CurrentHealth`) Damage))))
  (if (<= (`self.CurrentHealth`) 0.0)
    ;;[1 1 1] Смерть AI
    (set `self.IsDeath` true)
    (`SkeletalMeshComponent.SetAllBodiesSimulatePhysics` (`self.Mesh`) true)
    (`PrimitiveComponent.SetCollisionEnabled` (`self.CapsuleComponent`) "NoCollision")
    (`SceneComponent.SetVisibility` (`self.Widget`) false false)))

(event `EnableCombat`
  ;[1 1 1] Анимация атаки
  (`self.PlayAnimMontage` "/Game/BP/AI/Animation/AI_seat.AI_seat" -1.0))

(event `self.ReceiveTick`
  (params (DeltaSeconds :type "Float (single-precision)"))
  ;[1 1 1] При закате включить красные глаза
)

(fn `UserConstructionScript`)