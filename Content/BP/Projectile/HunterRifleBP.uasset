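; Hunter rifle weapon Blueprint that supplies the rifle's ammo, clip, damage and spread tuning.
; Its construction script runs the parent's, then overwrites those stat variables with rifle-specific defaults, including the spread range and recovery speed.
; The event graph holds only disabled placeholder events, so this file adds no runtime logic of its own.
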(fn `UserConstructionScript`
  (`parent.UserConstructionScript`)
  ;[1 1 1] Установка значений по умолчанию
  (set `self.MaxAmmo` 30)
  (set `self.CurrentAmmo` 5)
  (set `self.Damage` 100.0)
  (set `self.ClipSize` 5)
  (set `self.SpreadMin` 0.0)
  (set `self.SpreadMax` 0.3)
  (set `self.SpreadDecreaseSpeed` 0.25))