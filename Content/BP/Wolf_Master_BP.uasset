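; Wolf_Master_BP is the wolf character Blueprint, handling health, incoming damage and death state.
; On BeginPlay it fills health to maximum and registers itself as owner of the Wolf_UI in its widget component.
; The ITakeDamage event subtracts damage, except that a hit on the "Brust" bone prints "Head shot" and zeroes health.
; Health at or below zero only sets the IsDeath flag.
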(event `self.ReceiveBeginPlay`
  (set `self.CurrentHealth` (`self.MaxHealth`))
  (bind _aswolf_ui (cast `/Game/UI/Wolf_UI` (`WidgetComponent.GetUserWidgetObject` (`self.Widget`))))
  (set `/Game/UI/Wolf_UI.Owner` self _aswolf_ui))

(event `/Game/BP/TakeDAmage.iTakeDamage`
  (params (BoneName :type Name) (Damage :type "Float (single-precision)"))
  (if (== BoneName "Brust")
    (`KismetSystemLibrary.PrintString` "Head shot")
    (set `self.CurrentHealth` 0.0)
    (else
      (set `self.CurrentHealth` (- (`self.CurrentHealth`) Damage))))
  (if (<= (`self.CurrentHealth`) 0.0)
    (set `self.IsDeath` true)))

(fn `UserConstructionScript`)