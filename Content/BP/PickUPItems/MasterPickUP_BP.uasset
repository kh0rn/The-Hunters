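; Master pickup actor that the Hunter can inspect up close and collect as health, doll, ammo or knife.
; Sphere overlap shows a prompt widget and custom-depth highlight, enables input and registers the item with the player.
; A FlipFlop on Inspection first locks the player and lerps the item to their inspection point via Timeline, then collects it by type.
; Cancel frees the player and reverses the Timeline.
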(event `self.Sphere.OnComponentBeginOverlap`
  (params (OverlappedComponent :type "PrimitiveComponent Object Reference") (OtherActor :type "Actor Object Reference") (OtherComp :type "PrimitiveComponent Object Reference") (OtherBodyIndex :type Integer) (bFromSweep :type Boolean) (SweepResult :type "HitResult Structure (by ref)"))
  (bind _ashunter (cast `/Game/BP/Character/Hunter` OtherActor))
  (set `self.Player` _ashunter)
  (`SceneComponent.SetVisibility` (`self.Widget`) true false)
  (`PrimitiveComponent.SetRenderCustomDepth` (`self.StaticMesh`) true)
  (`PrimitiveComponent.SetRenderCustomDepth` (`self.SkeletalMesh`) true)
  (set `self.CanPick` true)
  (`self.EnableInput` (`GameplayStatics.GetPlayerController` 0))
  (set `/Game/BP/Character/Hunter.SetInspectionObject` self (`self.Player`)))

(event `self.Sphere.OnComponentEndOverlap`
  (params (OverlappedComponent :type "PrimitiveComponent Object Reference") (OtherActor :type "Actor Object Reference") (OtherComp :type "PrimitiveComponent Object Reference") (OtherBodyIndex :type Integer))
  (bind _ashunter (cast `/Game/BP/Character/Hunter` OtherActor))
  (set `self.Player` _ashunter)
  (`SceneComponent.SetVisibility` (`self.Widget`) false false)
  (`PrimitiveComponent.SetRenderCustomDepth` (`self.SkeletalMesh`) false)
  (`PrimitiveComponent.SetRenderCustomDepth` (`self.StaticMesh`) false)
  (set `/Game/BP/Character/Hunter.SetInspectionObject` null (`self.Player`)))

(event `InputAction|Cancel`
  (params (Key :type "Key Structure"))
  ;[1 1 1] Система пред просмотра айтемов
  (:`Pressed`
    (`self.FreePlayer`)
    (bind (_direction _moveactor) (`Timeline|Timeline_0` :!via `Reverse` :!label _label)
      (:`Update`
        (set `self.Moveactor` _moveactor)
        (`self.K2_SetActorLocationAndRotation` (`KismetMathLibrary.VLerp` (`self.InspectionObjectLocation`) (`SceneComponent.K2_GetComponentLocation` (`/Game/BP/Character/Hunter.InspectionLoc` (`self.Player`))) (`self.Moveactor`)) (`KismetMathLibrary.RLerp` (`self.InspectionObject`) (`self.K2_GetActorRotation`) (`self.Moveactor`)))))))

(event `InputAction|Inspection`
  (params (Key :type "Key Structure"))
  (bind _player (`self.Player`))
  (bind _player_2 (`self.Player`))
  (bind _player_3 (`self.Player`))
  (bind _player_4 (`self.Player`))
  (bind _player_5 (`self.Player`))
  (bind _maxammo (`/Game/BP/Weapons/MasterWeaponBP.MaxAmmo` (`/Game/BP/Character/Hunter.Rifle_BP` (`self.Player`))))
  (bind _returnvalue (+ (`self.PickupAmmo`) _maxammo))
  ;[1 1 1] Система пред просмотра айтемов
  (:`Pressed`
    (if (`self.CanPick`)
      (`/Engine/EditorBlueprintResources/StandardMacros.FlipFlop`
        (:`A`
          (set `/Game/BP/Character/Hunter.IsInspecting` true _player_5)
          (set `/Game/BP/Character/Hunter.StopMovement` true _player_5)
          (set `/Game/BP/Character/Hunter.AimWeapon` false _player_5)
          (if (`/Game/BP/Character/Hunter.EquipWeapon` _player_2)
            (`/Game/BP/Character/Hunter.Equip/UnEquip` _player_2))
          (set `self.InspectionObject` (`self.K2_GetActorRotation`))
          (set `self.InspectionObjectLocation` (`self.K2_GetActorLocation`))
          (goto _label))
        (:`B`
          (switch `/Game/BP/PickUPItems/ItemPickUp` (`self.ItemPickUp`)
            (:`NewEnumerator1`
              (bind _result (`/Engine/EditorBlueprintResources/StandardMacros.IncrementInt` (`/Game/BP/Character/Hunter.HealthPack` _player_3))
                (:`  `
                  (set `/Game/BP/Character/Hunter.HealthPack` _result _player_3)
                  (`self.K2_DestroyActor`)
                  (`self.FreePlayer` :!label _label_2))))
            (:`NewEnumerator2`
              (bind _result_2 (`/Engine/EditorBlueprintResources/StandardMacros.IncrementInt` (`/Game/BP/Character/Hunter.Doll` _player_4))
                (:`  `
                  (set `/Game/BP/Character/Hunter.Doll` _result_2 _player_4)
                  (`self.K2_DestroyActor`)
                  (goto _label_2))))
            (:`NewEnumerator3`
              (if (`KismetSystemLibrary.IsValid` (`/Game/BP/Character/Hunter.Rifle_BP` (`self.Player`)))
                (if (== (`self.PickupAmmo`) _maxammo)
                  (`KismetSystemLibrary.PrintString` "Full of ammo")
                  (else
                    (if (>= _returnvalue (`self.PickupAmmo`))
                      (set `/Game/BP/Weapons/MasterWeaponBP.MaxAmmo` (`self.PickupAmmo`) (`/Game/BP/Character/Hunter.Rifle_BP` (`self.Player`)))
                      (else
                        (set `/Game/BP/Weapons/MasterWeaponBP.MaxAmmo` _returnvalue (`/Game/BP/Character/Hunter.Rifle_BP` (`self.Player`)))))
                    (`GameplayStatics.PlaySound2D` null)
                    (`self.K2_DestroyActor`)
                    (`self.FreePlayer`)))))
            (:`NewEnumerator4`
              (bind _result_3 (`/Engine/EditorBlueprintResources/StandardMacros.IncrementInt` (`/Game/BP/Character/Hunter.Knife` _player))
                (:`  `
                  (set `/Game/BP/Character/Hunter.Knife` _result_3 _player)
                  (`self.K2_DestroyActor`)
                  (`self.FreePlayer`))))))))))

(fn `UserConstructionScript`)