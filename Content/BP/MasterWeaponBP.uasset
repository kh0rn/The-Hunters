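; Master weapon Blueprint that handles the player's rifle firing, ammo and aim spread, using ammo counts stored on the player's RifleBP.
; A Gate with a retriggerable delay repeats fire while held, line tracing from the ADS component with sound, montage and impact particles, but no damage.
; Shots increase spread, which Tick decays, though the trace ignores it.
; Release triggers auto-reload on empty, but Reloding's always-true branch leaves WeaponReload unreachable.
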(event `self.ReceiveBeginPlay`
  ;[1 1 1] Обращение к переменной player
  (bind _asplayer_character (cast `/Game/BP/PlayerCharacter` (`GameplayStatics.GetPlayerCharacter` 0)))
  (bind _output_get (set `self.Player` _asplayer_character))
  (`KismetArrayLibrary.Array_Add` (`self.IgnoreActor`) _output_get)
  (`KismetArrayLibrary.Array_Add` (`self.IgnoreActor`) (`/Game/BP/PlayerCharacter.Rifle_BP` (`self.Player`))))

(event `StartFire`
  (bind _rifle_bp (`/Game/BP/PlayerCharacter.Rifle_BP` (`self.Player`)))
  (bind _ads (`/Game/BP/PlayerCharacter.ADS` (`self.Player`)))
  (bind _returnvalue (`SceneComponent.K2_GetComponentLocation` _ads))
  (bind _currentammo (`/Game/BP/MasterWeaponBP.CurrentAmmo` _rifle_bp))
  (`|ExecutionSequence`
    (:`then_0`
      (goto _label :!via `Open`))
    (:`then_1`
      (`/Engine/EditorBlueprintResources/StandardMacros.Gate` true :!label _label
        (:`Exit`
          (`|ExecutionSequence`
            (:`then_0`
              (`KismetSystemLibrary.RetriggerableDelay` 5.0)
              (goto _label))
            (:`then_1`
              (if (<= (`/Game/BP/MasterWeaponBP.CurrentAmmo` (`/Game/BP/PlayerCharacter.Rifle_BP` (`self.Player`))) 0)
                (`KismetSystemLibrary.PrintString` "Out of Ammo")
                (else
                  (bind (_outhit _returnvalue_2) (`KismetSystemLibrary.LineTraceSingle` _returnvalue (+ _returnvalue (* (`SceneComponent.GetForwardVector` _ads) 15000.0)) "TraceTypeQuery1" false (`self.IgnoreActor`) "ForDuration"))
                  (if _returnvalue_2
                    _
                    (else
                      _))
                  (`GameplayStatics.PlaySound2D` null)
                  (`Character.PlayAnimMontage` (`self.Player`) "/Game/SG_Main/SG_Character/Animations/HipRifleAim.HipRifleAim" 1.0 "None")
                  (set `/Game/BP/MasterWeaponBP.CurrentAmmo` (- _currentammo 1) _rifle_bp)
                  (`KismetSystemLibrary.PrintString` (`KismetStringLibrary.Conv_IntToString` _currentammo))
                  (`GameplayStatics.SpawnEmitterAtLocation` "/Game/InfinityBladeEffects/Effects/FX_Mobile/Impacts/P_Impact_Enemy_Base.P_Impact_Enemy_Base" (`.Location` (`GameplayStatics.BreakHitResult` _outhit)))
                  (`self.IncreaseSpread` 0.3))))))))))

(event `StopFire`
  (goto _label :!via `Close`))

(event `FirePress`
  (set `self.CanFire` true)
  (if (not (`self.IsReloding`))
    (`self.StartFire`)))

(event `FireRelease`
  (set `self.CanFire` false)
  (`self.StopFire`)
  (`self.AutoReload`))

(event `AutoReload`
  (if (== (`/Game/BP/MasterWeaponBP.CurrentAmmo` (`/Game/BP/PlayerCharacter.Rifle_BP` (`self.Player`))) 0)
    (if (== (`/Game/BP/MasterWeaponBP.MaxAmmo` (`/Game/BP/PlayerCharacter.Rifle_BP` (`self.Player`))) 0)
      (`KismetSystemLibrary.PrintString` "Find ammo")
      (else
        (set `self.IsReloding` true)
        (`self.Reloding`)
        (`KismetSystemLibrary.Delay` 10.0) ; Reload animation
        (set `self.IsReloding` false)))))

(event `self.ReceiveTick`
  (params (DeltaSeconds :type "Float (single-precision)"))
  ;[1 1 1] Уменьшение разброса прицела по прошедствию времени
  (set `self.DeltaTime` DeltaSeconds)
  (if (>= (`self.SpreadCurrent`) (`self.SpreadMin`))
    (`self.DecreaseSpread` (* (`self.DeltaTime`) (`self.SpreadDecreaseSpeed`)))))

(event `Reloding`
  (bind _rifle_bp (`/Game/BP/PlayerCharacter.Rifle_BP` (`self.Player`)))
  (if true
    (`KismetSystemLibrary.PrintString` "Find Ammo")
    (elif (== (`/Game/BP/MasterWeaponBP.CurrentAmmo` _rifle_bp) (`/Game/BP/MasterWeaponBP.ClipSize` _rifle_bp))
      (`KismetSystemLibrary.PrintString` "Find Ammo")
      (else
        (bind _output_get (set `self.IsReloding` true))
        (if _output_get
          (`self.WeaponReload`)
          (`KismetSystemLibrary.Delay` 10.0)
          (set `self.IsReloding` false))))))

(event `WeaponReload`
  (bind _neadedammo (`self.NeadedAmmo`))
  (bind _rifle_bp (`/Game/BP/PlayerCharacter.Rifle_BP` (`self.Player`)))
  (bind _rifle_bp_2 (`/Game/BP/PlayerCharacter.Rifle_BP` (`self.Player`)))
  (bind _rifle_bp_3 (`/Game/BP/PlayerCharacter.Rifle_BP` (`self.Player`)))
  (bind _maxammo (`/Game/BP/MasterWeaponBP.MaxAmmo` (`/Game/BP/PlayerCharacter.Rifle_BP` (`self.Player`))))
  (if (not (`self.CanFire`))
    (`Character.PlayAnimMontage` (`self.Player`) null 1.0 "None")
    (if (> (`/Game/BP/MasterWeaponBP.MaxAmmo` (`/Game/BP/PlayerCharacter.Rifle_BP` (`self.Player`))) 0)
      (set `self.NeadedAmmo` (- (`/Game/BP/MasterWeaponBP.ClipSize` _rifle_bp) (`/Game/BP/MasterWeaponBP.CurrentAmmo` _rifle_bp)))
      (if (<= _maxammo _neadedammo)
        (set `/Game/BP/MasterWeaponBP.CurrentAmmo` (+ (`/Game/BP/MasterWeaponBP.MaxAmmo` _rifle_bp_2) (`/Game/BP/MasterWeaponBP.CurrentAmmo` _rifle_bp_2)) (`/Game/BP/PlayerCharacter.Rifle_BP` (`self.Player`)))
        (else
          (set `/Game/BP/MasterWeaponBP.MaxAmmo` (- _maxammo _neadedammo) _rifle_bp_3)
          (set `/Game/BP/MasterWeaponBP.CurrentAmmo` (`/Game/BP/MasterWeaponBP.ClipSize` _rifle_bp_3) _rifle_bp_3))))))

(fn `DecreaseSpread`
  (params (DecreaseAmmount :type "Float (double-precision)"))
  (bind _returnvalue (- (`self.SpreadCurrent`) DecreaseAmmount))
  (if (<= _returnvalue (`self.SpreadMin`))
    (set `self.SpreadCurrent` (`self.SpreadMin`))
    (else
      (set `self.SpreadCurrent` _returnvalue)))
  (return))

(fn `IncreaseSpread`
  (params (IncreaseAmount :type "Float (double-precision)"))
  (bind _returnvalue (+ IncreaseAmount (`self.SpreadCurrent`)))
  (if (>= _returnvalue (`self.SpreadMax`))
    (set `self.SpreadCurrent` (`self.SpreadMax`))
    (else
      (set `self.SpreadCurrent` _returnvalue)))
  (return))

(fn `UserConstructionScript`)