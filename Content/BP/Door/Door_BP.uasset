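; Interactive door actor that the Hunter can open only while carrying at least one Doll or Knife.
; Box overlap toggles an outline via custom depth and front/back prompt widgets, sets the prompt text and arms the Inspection input.
; That input toggles timelines that swing the actor's yaw from its starting rotation; leaving the box closes an open door.
; Sounds fire on every timeline update, not once per swing.
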(event `self.ReceiveBeginPlay`
  (set `self.CurrentRotation` (`self.K2_GetActorRotation`)))

(event `self.Box.OnComponentBeginOverlap`
  (params (OverlappedComponent :type "PrimitiveComponent Object Reference") (OtherActor :type "Actor Object Reference") (OtherComp :type "PrimitiveComponent Object Reference") (OtherBodyIndex :type Integer) (bFromSweep :type Boolean) (SweepResult :type "HitResult Structure (by ref)"))
  (bind _hunter (`self.Hunter`))
  ;[1 1 1] Игрок подходит к двери, если у игрока есть ключи доступа то дверь можно открыть
  (bind _ashunter (cast `/Game/BP/Character/Hunter` OtherActor))
  (set `self.Hunter` _ashunter)
  (`PrimitiveComponent.SetRenderCustomDepth` (`self.StaticMesh`) true)
  (`SceneComponent.SetVisibility` (`self.WidgetFront`) true false)
  (`SceneComponent.SetVisibility` (`self.WidgetBack`) true false)
  ;;[1 1 1] Есть ключи, дверь можно откртыть
  (if (or (>= (`/Game/BP/Character/Hunter.Doll` _hunter) 1) (>= (`/Game/BP/Character/Hunter.Knife` _hunter) 1))
    (bind _asdoor_ui (cast `/Game/UI/Env/Door_UI` (`WidgetComponent.GetUserWidgetObject` (`self.WidgetFront`))))
    (set `/Game/UI/Env/Door_UI.KeyText` "Open Door [F]" _asdoor_ui)
    (`self.EnableInput` (`GameplayStatics.GetPlayerController` 0))
    (set `self.CanDoorOpen` true)
    (else
      ;;[1 1 1] Нет ключей дверь не откроется
      (bind _asdoor_ui_2 (cast `/Game/UI/Env/Door_UI` (`WidgetComponent.GetUserWidgetObject` (`self.WidgetFront`))))
      (set `/Game/UI/Env/Door_UI.KeyText` "Find Doll or Knife to  \nOpen" _asdoor_ui_2)
      (set `self.CanDoorOpen` false))))

(event `self.Box.OnComponentEndOverlap`
  (params (OverlappedComponent :type "PrimitiveComponent Object Reference") (OtherActor :type "Actor Object Reference") (OtherComp :type "PrimitiveComponent Object Reference") (OtherBodyIndex :type Integer))
  ;[1 1 1] Игрок отошел от двери
  (bind _ashunter (cast `/Game/BP/Character/Hunter` OtherActor))
  (set `self.Hunter` _ashunter)
  (`PrimitiveComponent.SetRenderCustomDepth` (`self.StaticMesh`) false)
  (`SceneComponent.SetVisibility` (`self.WidgetFront`) false false)
  (`SceneComponent.SetVisibility` (`self.WidgetBack`) false false)
  (set `self.CanDoorOpen` false)
  ;[1 1 1] Закрытие двери
  (if (`self.IsDoorOpen`)
    (bind (_direction _opendoor) (`Timeline|Timeline_0` :!via `ReverseFromEnd`)
      (:`Update`
        (`self.K2_SetActorRelativeRotation` (`KismetMathLibrary.MakeRotator` 0.0 0.0 (+ (.yaw (`self.CurrentRotation`)) _opendoor)))
        (set `self.IsDoorOpen` false)
        (`GameplayStatics.PlaySound2D` "/Game/Audio/CloseDoor.CloseDoor")))))

(event `InputAction|Inspection`
  (params (Key :type "Key Structure"))
  ;[1 1 1] Взаимодействие с дверью
  (:`Pressed`
    (if (`self.CanDoorOpen`)
      (if (`self.IsDoorOpen`)
        ;;[1 1 1] Закрытие двери
        (bind (_direction _opendoor) (`Timeline|CloseDoor` :!via `ReverseFromEnd`)
          (:`Update`
            (`self.K2_SetActorRelativeRotation` (`KismetMathLibrary.MakeRotator` 0.0 0.0 (+ (.yaw (`self.CurrentRotation`)) _opendoor)))
            (set `self.IsDoorOpen` false)
            (`GameplayStatics.PlaySound2D` "/Game/Audio/CloseDoor.CloseDoor")))
        (else
          ;;[1 1 1] Открытие двери
          (bind (_direction_2 _opendoor_2) (`Timeline|OpenDoor` :!via `PlayFromStart`)
            (:`Update`
              (`self.K2_SetActorRelativeRotation` (`KismetMathLibrary.MakeRotator` 0.0 0.0 (+ (.yaw (`self.CurrentRotation`)) _opendoor_2)))
              (set `self.IsDoorOpen` true)
              (`GameplayStatics.PlaySound2D` "/Game/Audio/Open.Open"))))))))

(fn `UserConstructionScript`)